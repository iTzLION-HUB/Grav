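; BP_DamageVol is a damage volume that periodically hurts the first player's character while it overlaps the Box.
; A one-second looping timer runs on authority, checking the box's overlapping actors against the character cached at BeginPlay.
; On a match it self-applies GE_DamageVol through the character's Ability System, passing DamageAmt as a SetByCaller magnitude.
; Each hit also reports the volume to the character's quest system as an interaction.
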(event `self.ReceiveBeginPlay`
  (bind _asbp_first_person_character (cast `/Game/FirstPerson/Blueprints/BP_FirstPersonCharacter` (`GameplayStatics.GetPlayerCharacter` 0)))
  (set `self. First Person Character` _asbp_first_person_character)
  (`KismetSystemLibrary.K2_SetTimerDelegate` (delegate `DamageTick`) 1.0 true))

(event `DamageTick`
  (`/Engine/EditorBlueprintResources/ActorMacros.Switch Has Authority`
    (:`Authority`
      (for _array_element (`PrimitiveComponent.GetOverlappingActors` (`self.Box`) null)
        (if (== (`self. First Person Character`) _array_element)
          (bind _returnvalue (`AbilitySystemBlueprintLibrary.GetAbilitySystemComponent` _array_element))
          (bind _returnvalue_2 (`AbilitySystemBlueprintLibrary.AssignTagSetByCallerMagnitude` (`AbilitySystemComponent.MakeOutgoingSpec` _returnvalue "/Game/GameplayAbility/Abillities/DamageVolume/GE_DamageVol.GE_DamageVol_C" 0.0 (`AbilitySystemComponent.MakeEffectContext` _returnvalue)) (struct :`TagName` "Damage.SetByCaller") (`self.DamageAmt`)))
          (`AbilitySystemComponent.BP_ApplyGameplayEffectSpecToSelf` _returnvalue _returnvalue_2)
          (`/Game/Blueprint/ObjectiveSystem/Data/AC_QuestSystem.InteractedWithActor` (`/Game/FirstPerson/Blueprints/BP_FirstPersonCharacter.AC_QuestSystem` (`self. First Person Character`)) self))))))

(fn `UserConstructionScript`)