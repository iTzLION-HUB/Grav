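; Gameplay ability that throws a physics-simulated smoke grenade from the first-person character.
; On activation it checks cost and cooldown, commits, and computes a spawn point just ahead of the character's GrenadeLocation.
; The authority spawns BP_SmokeGrenade and launches it along the actor's forward vector.
; SpawnRotation, a camera trace for reticle-aligned aiming, is never called, so the spawn's Direction is not updated.
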(event `self.K2_ActivateAbility`
  (bind _firstpersoncharacter (`self.FirstPersonCharacter`))
  ;[1 1 1] Determine if Ability can be activated
  (bind _asbp_first_person_character (cast `/Game/FirstPerson/Blueprints/BP_FirstPersonCharacter` (`self.GetAvatarActorFromActorInfo`)))
  (set `self.FirstPersonCharacter` _asbp_first_person_character)
  (bind _asbp_first_person_player_controller (cast `/Game/FirstPerson/Blueprints/BP_FirstPersonPlayerController` (`GameplayStatics.GetPlayerController` 0)))
  (set `self.Player Controller` _asbp_first_person_player_controller)
  (bind _returnvalue (`self.K2_CheckAbilityCost`))
  (bind _returnvalue_2 (`self.K2_CheckAbilityCooldown`))
  (if (and _returnvalue _returnvalue_2)
    (`self.K2_CommitAbility`)
    ;[1 1 1] Spawn and Targeting Logic
    (set `self.Location` (+ (`SceneComponent.K2_GetComponentLocation` (`/Game/FirstPerson/Blueprints/BP_FirstPersonCharacter.GrenadeLocation` _firstpersoncharacter)) (* (`Actor.GetActorForwardVector` _firstpersoncharacter) 20.0) (* (`Actor.GetActorUpVector` _firstpersoncharacter) 25.0)))
    (`self.K2_HasAuthority`
      (:`True`
        (bind _returnvalue_3 (`|SpawnActorFromClass` "/Game/GameplayAbility/Abillities/Smoke/BP_SmokeGrenade.BP_SmokeGrenade_C" (`KismetMathLibrary.MakeTransform` (`self.Location`) (`self.Direction`)) "AlwaysSpawn" "MultiplyWithRoot" null 2.0 false null))
        (bind _sphere (`/Game/GameplayAbility/Abillities/Smoke/BP_SmokeGrenade.Sphere` _returnvalue_3))
        (`PrimitiveComponent.SetSimulatePhysics` _sphere true)
        (`PrimitiveComponent.SetPhysicsLinearVelocity` _sphere (* (`KismetMathLibrary.GetForwardVector` (`Actor.K2_GetActorRotation` (`self.FirstPersonCharacter`))) (`self.ImpluseStrength`)) false "None")
        (`self.K2_EndAbility`)))
    (else
      (`self.K2_EndAbility`))))