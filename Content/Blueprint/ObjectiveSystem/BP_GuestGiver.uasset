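; BP_GuestGiver is an interactable quest giver actor that presents its Quests list to the player.
; Interact toggles a WBP_QuestGiver menu, passing it a self reference and each quest's details while switching mouse cursor and input mode.
; CloseWidget jumps into the same teardown branch, restoring game-only input.
; A sphere collision shows or hides the actor's Widget component as the player character enters or leaves range.
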(event `/Game/Blueprint/ObjectiveSystem/Data/BPI_Quest.Interact`
  (bind _returnvalue (`GameplayStatics.GetPlayerController` 0))
  ;[0 1 0.9865 0.1] OnInteract
  (if (not (`self.WidgetActive`))
    (bind _returnvalue_2 (`|CreateWidget` "/Game/UI/Quest/WBP_QuestGiver.WBP_QuestGiver_C"))
    (bind _output_get (set `self.WBP_Quest` _returnvalue_2))
    (`UserWidget.AddToViewport` _output_get 0)
    (set `self.WidgetActive` true)
    (set `PlayerController.bShowMouseCursor` true _returnvalue)
    (`WidgetBlueprintLibrary.SetInputMode_GameAndUIEx` _returnvalue (`self.WBP_Quest`))
    (set `/Game/UI/Quest/WBP_QuestGiver.QuestGiverBP` self (`self.WBP_Quest`))
    (for _array_element (`self.Quests`)
      (`/Game/UI/Quest/WBP_QuestGiver.AddQuestDetails` (`self.WBP_Quest`) _array_element))
    (else
      (`Widget.RemoveFromParent` (`self.WBP_Quest`) :!label _label)
      (set `self.WBP_Quest` null)
      (set `self.WidgetActive` false)
      (set `PlayerController.bShowMouseCursor` false _returnvalue)
      (`WidgetBlueprintLibrary.SetInputMode_GameOnly` _returnvalue))))

(event `CloseWidget`
  ;[0 1 0.9865 0.1] OnInteract
  (goto _label))

(event `self.SphereCollision.OnComponentBeginOverlap`
  (params (OverlappedComponent :type "PrimitiveComponent Object Reference") (OtherActor :type "Actor Object Reference") (OtherComp :type "PrimitiveComponent Object Reference") (OtherBodyIndex :type Integer) (bFromSweep :type Boolean) (SweepResult :type "HitResult Structure (by ref)"))
  ;[0.4028 0.2448 1 0.1] Seting Widget Visibility
  (if (== OtherActor (`GameplayStatics.GetPlayerCharacter` 0))
    (`SceneComponent.SetVisibility` (`self.Widget`) true false)))

(event `self.SphereCollision.OnComponentEndOverlap`
  (params (OverlappedComponent :type "PrimitiveComponent Object Reference") (OtherActor :type "Actor Object Reference") (OtherComp :type "PrimitiveComponent Object Reference") (OtherBodyIndex :type Integer))
  ;[0.4028 0.2448 1 0.1] Seting Widget Visibility
  (if (== (`GameplayStatics.GetPlayerCharacter` 0) OtherActor)
    (`SceneComponent.SetVisibility` (`self.Widget`) false false)))

(fn `UserConstructionScript`)