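; Quest system component that tracks the active quest's objectives and shows them on an objective HUD.
; It creates the HUD hidden on BeginPlay, then events fill in the quest title and objectives.
; Interact and chest-open events mark objectives completed by reference, with interactions completing one while its actor list remains non-empty after removal.
; A completion counter clears the quest and plays the HUD animation once it reaches the objective count.
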(event `self.ReceiveBeginPlay`
  ;[1 0 0.298 0.2] BeginPlay
  (bind _returnvalue (`|CreateWidget` "/Game/UI/Quest/WBP_ObjectiveHUD.WBP_ObjectiveHUD_C"))
  (bind _output_get (set `self.WBP_QuestHUD` _returnvalue))
  (`UserWidget.AddToViewport` _output_get 0)
  (`/Game/UI/Quest/WBP_ObjectiveHUD.HidePanel` _output_get))

(event `SetActiveQuestText`
  (bind _activequest_name (break `/Game/Blueprint/ObjectiveSystem/Data/FStruct_Quest` (`self.ActiveQuest`)))
  ;[1 0.1094 0.3548 0.2] SetActiveQuest
  (`TextBlock.SetText` (`/Game/UI/Quest/WBP_ObjectiveHUD.TxtBlock_ObjectiveTitle` (`self.WBP_QuestHUD`)) _activequest_name)
  (`/Game/UI/Quest/WBP_ObjectiveHUD.ShowPanel` (`self.WBP_QuestHUD`)))

(event `SetObjectives`
  (bind (_activequest_name _activequest_description _activequest_completed _activequest_secondary _activequest_objective) (break `/Game/Blueprint/ObjectiveSystem/Data/FStruct_Quest` (`self.ActiveQuest`)))
  ;[0 1 0.3867 0.2] SetObjective
  (`/Game/UI/Quest/WBP_ObjectiveHUD.FillObjectives` (`self.WBP_QuestHUD`) _activequest_objective))

(event `InteractedWithActor`
  (params (Actor :type "Actor Object Reference"))
  (bind (_activequest_name _activequest_description _activequest_completed _activequest_secondary _activequest_objective) (break `/Game/Blueprint/ObjectiveSystem/Data/FStruct_Quest` (`self.ActiveQuest`)))
  ;[0 0.482 1 0.2] Interacting Quest
  (for _array_element _activequest_objective
    (bind (_name _completed _actorinteract _chesttoopen _ischestobjective) (break `/Game/Blueprint/ObjectiveSystem/Data/FStruct_QuestObjective` _array_element))
    (if (and (not _completed) (> (`KismetArrayLibrary.Array_Length` _actorinteract) 0))
      (`KismetArrayLibrary.Array_RemoveItem` _actorinteract Actor)
      (if (!= (`KismetArrayLibrary.Array_Length` _actorinteract) 0)
        (`|VariableSetRef` _array_element (make `/Game/Blueprint/ObjectiveSystem/Data/FStruct_QuestObjective` _name true _actorinteract _chesttoopen _ischestobjective))
        (`/Game/UI/Quest/WBP_ObjectiveHUD.CompleteObjective` (`self.WBP_QuestHUD`) _array_element)
        (`self.AllObjectiveCompleted`)))))

(event `OpenChest`
  (params (Chest :type "Actor Object Reference"))
  (bind (_activequest_name _activequest_description _activequest_completed _activequest_secondary _activequest_objective) (break `/Game/Blueprint/ObjectiveSystem/Data/FStruct_Quest` (`self.ActiveQuest`)))
  ;[0 1 0.5218 0.2] Opening Chest
  (for _array_element _activequest_objective
    (bind (_name _completed _actorinteract _chesttoopen _ischestobjective) (break `/Game/Blueprint/ObjectiveSystem/Data/FStruct_QuestObjective` _array_element))
    (if (and _ischestobjective (== _chesttoopen Chest))
      (`|VariableSetRef` _array_element (make `/Game/Blueprint/ObjectiveSystem/Data/FStruct_QuestObjective` _name true _actorinteract null _ischestobjective))
      (`/Game/UI/Quest/WBP_ObjectiveHUD.CompleteObjective` (`self.WBP_QuestHUD`) _array_element)
      (`self.AllObjectiveCompleted`))))

(event `AllObjectiveCompleted`
  (bind (_activequest_name _activequest_description _activequest_completed _activequest_secondary _activequest_objective) (break `/Game/Blueprint/ObjectiveSystem/Data/FStruct_Quest` (`self.ActiveQuest`)))
  ;[0.4166 0 1 0.2] OnQuestComplete
  (`/Engine/EditorBlueprintResources/StandardMacros.IncrementInt` (`self.ObjectivesCompleted`)
    (:`  `
      (if (>= (`self.ObjectivesCompleted`) (`KismetArrayLibrary.Array_Length` _activequest_objective))
        (set `self.ActiveQuest` (struct))
        (set `self.ObjectivesCompleted` 0)
        (`/Game/UI/Quest/WBP_ObjectiveHUD.PlayQuestCompletedAnim` (`self.WBP_QuestHUD`))))))