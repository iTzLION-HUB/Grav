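; BP_LocateChest is a trigger volume that reports to the quest system when the local player reaches it.
; BeginPlay caches the first-person character, and a box overlap by that character calls InteractedWithActor on its quest component with this actor.
; The construction script sizes the box from an InBoxExtent variable.
; An authority-only FoundActor event loops over overlapping actors but does nothing with them.
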(event `self.ReceiveBeginPlay`
  (bind _asbp_first_person_character (cast `/Game/FirstPerson/Blueprints/BP_FirstPersonCharacter` (`GameplayStatics.GetPlayerCharacter` 0)))
  (set `self. First Person Character` _asbp_first_person_character))

(event `FoundActor`
  (`/Engine/EditorBlueprintResources/ActorMacros.Switch Has Authority`
    (:`Authority`
      (for _ (`PrimitiveComponent.GetOverlappingActors` (`self.Box`) null)
        _))))

(event `self.Box.OnComponentBeginOverlap`
  (params (OverlappedComponent :type "PrimitiveComponent Object Reference") (OtherActor :type "Actor Object Reference") (OtherComp :type "PrimitiveComponent Object Reference") (OtherBodyIndex :type Integer) (bFromSweep :type Boolean) (SweepResult :type "HitResult Structure (by ref)"))
  (if (== (`self. First Person Character`) OtherActor)
    (`/Game/Blueprint/ObjectiveSystem/Data/AC_QuestSystem.InteractedWithActor` (`/Game/FirstPerson/Blueprints/BP_FirstPersonCharacter.AC_QuestSystem` (`self. First Person Character`)) self)))

(fn `UserConstructionScript`
  (`BoxComponent.SetBoxExtent` (`self.Box`) (`self.In Box Extent`) true))