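; BP_Chest is a chest that can be opened once and reports its opening to the player's quest system.
; OpenChest checks the AlreadyOpen flag, casts player 0's character to BP_FirstPersonCharacter, and plays a non-looping open animation on ChestModel.
; It then passes itself to the character's ACQuestSystem component, then sets and returns the flag.
; The event graph and construction script are empty, so opening relies on an external call.
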(event `self.ReceiveBeginPlay`)

(fn `OpenChest`
  (returns (Completed :type Boolean))
  (if (not (`self.AlreadyOpen`))
    (bind _asbp_first_person_character (cast `/Game/FirstPerson/Blueprints/BP_FirstPersonCharacter` (`GameplayStatics.GetPlayerCharacter` 0)))
    (set `self.FirstPersonCharacter` _asbp_first_person_character)
    (`SkeletalMeshComponent.PlayAnimation` (`self.ChestModel`) "/Game/Blueprint/Chest/Mesh/Chest_Anim_Open.Chest_Anim_Open" false)
    (`/Game/Blueprint/ObjectiveSystem/Data/AC_QuestSystem.OpenChest` (`/Game/FirstPerson/Blueprints/BP_FirstPersonCharacter.AC_QuestSystem` (`self.FirstPersonCharacter`)) self)
    (bind _output_get (set `self.AlreadyOpen` true))
    (return _output_get)))

(fn `UserConstructionScript`)