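; Base destructible actor that uses the Gameplay Ability System for health, shaking when its health changes and destroying itself at zero.
; On BeginPlay it applies GE_InitHealthSet with SetByCaller magnitudes, setting health and max health from StartingHealth and leaving shield empty.
; OnHealthChanged calls ShakeBB while health remains, briefly tilting the static mesh and back after a short delay, otherwise it destroys the actor.
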(event `self.ReceiveBeginPlay`
  (bind _abilitysystemcomponent (`self.AbilitySystemComponent`))
  (bind _startinghealth (`self.StartingHealth`))
  ;[1 0 0.1676 0.2] Init Attribute
  (bind _returnvalue (`AbilitySystemBlueprintLibrary.AssignTagSetByCallerMagnitude` (`AbilitySystemComponent.MakeOutgoingSpec` :`self` _abilitysystemcomponent :`GameplayEffectClass` "/Game/GameplayAbility/Effects/GE_InitHealthSet.GE_InitHealthSet_C") (struct :`TagName` "HealthSet.Init.MaxHealth") _startinghealth))
  (bind _returnvalue_2 (`AbilitySystemBlueprintLibrary.AssignTagSetByCallerMagnitude` _returnvalue (struct :`TagName` "HealthSet.Init.Health") _startinghealth))
  (bind _returnvalue_3 (`AbilitySystemBlueprintLibrary.AssignTagSetByCallerMagnitude` _returnvalue_2 (struct :`TagName` "HeatlhSet.Init.MaxShield")))
  (bind _returnvalue_4 (`AbilitySystemBlueprintLibrary.AssignTagSetByCallerMagnitude` _returnvalue_3 (struct :`TagName` "HeatlhSet.Init.Shield")))
  (`AbilitySystemComponent.BP_ApplyGameplayEffectSpecToSelf` _abilitysystemcomponent _returnvalue_4))

(event `self.OnHealthChanged`
  (params (OldValue :type "Float (single-precision)") (NewValue :type "Float (single-precision)"))
  ;[0 1 0.5553] OnAttributeChanged
  (if (> NewValue 0.0)
    (`self.ShakeBB`)
    (else
      (`self.K2_DestroyActor`))))

(event `ShakeBB`
  ;[0 1 0.5553] OnAttributeChanged
  (`SceneComponent.K2_AddLocalRotation` (`self.StaticMeshComponent`) (struct :`Yaw` 5.0) false true)
  (`KismetSystemLibrary.Delay` 0.05)
  (`SceneComponent.K2_AddLocalRotation` (`self.StaticMeshComponent`) (struct :`Yaw` -5.0) false true))

(fn `UserConstructionScript`)